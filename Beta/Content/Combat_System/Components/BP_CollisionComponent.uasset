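; BP_CollisionComponent is a combat component that detects hits along a socketed mesh while collision is activated.
; Each tick while enabled, it runs a multi sphere trace for objects between start and end sockets on the assigned mesh, skipping ignored actors.
; An already-hit list, cleared on each activation, ensures each actor triggers the OnHit dispatcher only once per activation.
; Setters and getters expose the mesh, last hit, hit list and ignore list.
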(event `Activate Collision`
  (`self.Clear Hit Actors`)
  (set `self.isCollisionEnabled?` true))

(event `Deactivate Collision`
  (set `self.isCollisionEnabled?` false))

(event `Collision Trace`
  (bind _collisionmeshcomponent (`self.CollisionMeshComponent`))
  (bind _outhits (`KismetSystemLibrary.SphereTraceMultiForObjects` (`SceneComponent.GetSocketLocation` _collisionmeshcomponent (`self.Start Socket Name`)) (`SceneComponent.GetSocketLocation` _collisionmeshcomponent (`self.End Socket Name`)) (`self.TraceRadius`) (`self.Collision Object Types`) false (`self.ActorstoIgnore`) (`self.Draw Debug Type`)))
  (for _array_element _outhits
    (bind _output_get (set `self.LastHit` _array_element))
    (bind (_bblockinghit _binitialoverlap _time _distance _location _impactpoint _normal _impactnormal _physmat _hitactor) (`GameplayStatics.BreakHitResult` _output_get))
    (if (not (`KismetArrayLibrary.Array_Contains` (`self.AllreadyHitActors`) _hitactor))
      (bind _output_get_2 (set `self.Hit Actor` _hitactor))
      (`KismetArrayLibrary.Array_Add` (`self.AllreadyHitActors`) _output_get_2)
      (`self.OnHit` (`self.LastHit`)))))

(event `Clear Hit Actors`
  (`KismetArrayLibrary.Array_Clear` (`self.AllreadyHitActors`)))

(event `self.ReceiveTick`
  (params (DeltaSeconds :type "Float (single-precision)"))
  (if (`self.isCollisionEnabled?`)
    (`self.Collision Trace`)))

(event `SetCollisionMesh`
  (params (MeshComponent :type "PrimitiveComponent Object Reference"))
  (set `self.CollisionMeshComponent` MeshComponent))

(fn `AddActorToIgnore`
  (params (isActor :type "Actor Object Reference (by ref)"))
  (`KismetArrayLibrary.Array_AddUnique` (`self.ActorstoIgnore`) isActor))

(fn `GetActorsToIgnore`
  (returns (ReturnValue :type "Array of Actor Object Reference"))
  (return (`self.ActorstoIgnore`)))

(fn `GetAllreadyHitActors`
  (returns (ReturnValue :type "Array of Actor Object Reference"))
  (return (`self.AllreadyHitActors`)))

(fn `GetCollisionMeshComponent`
  (returns (ReturnValue :type "PrimitiveComponent Object Reference"))
  (return (`self.CollisionMeshComponent`)))

(fn `GetLastHit`
  (returns (ReturnValue :type "HitResult Structure"))
  (return (`self.LastHit`)))

(fn `is Collision Enabled?`
  (returns (ReturnValue :type Boolean))
  (return (`self.isCollisionEnabled?`)))

(fn `RemoveActorToIgnore`
  (params (ActorToRemove :type "Actor Object Reference (by ref)"))
  (`KismetArrayLibrary.Array_RemoveItem` (`self.ActorstoIgnore`) ActorToRemove))